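; Locked dungeon door that spends one of the player's keys and swings open when the custom third-person character enters its trigger sphere.
; With a key, it plays a hinge sound and a timeline rotates the door pivot, destroying the sphere when finished.
; Without keys, it prints a warning and plays a throttled locked sound if never unlocked.
; Leaving the sphere stops the timeline, and re-entering with keys spends another and restarts it.
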(event `self.Sphere.OnComponentBeginOverlap`
  (params (OverlappedComponent :type "PrimitiveComponent Object Reference") (OtherActor :type "Actor Object Reference") (OtherComp :type "PrimitiveComponent Object Reference") (OtherBodyIndex :type Integer) (bFromSweep :type Boolean) (SweepResult :type "HitResult Structure (by ref)"))
  (bind _asbp_third_person_character_custom (cast `/Game/Blueprints/BP_ThirdPersonCharacterCustom` OtherActor))
  (bind _key_count (`/Game/Blueprints/BP_ThirdPersonCharacterCustom.Key Count` _asbp_third_person_character_custom))
  (if (> _key_count 0)
    (set `/Game/Blueprints/BP_ThirdPersonCharacterCustom.Key Count` (- _key_count 1) _asbp_third_person_character_custom) ; Remove a Key, then open door.
    (`GameplayStatics.PlaySoundAtLocation` "/Game/Audio/Door_hinge_sounds_2_Cue.Door_hinge_sounds_2_Cue" (`SceneComponent.K2_GetComponentLocation` (`self.DefaultSceneRoot`)) (struct) 1.0 1.0 0.0 null null null null)
    (bind (_direction _newtrack_0) (`Timeline|Timeline` :!via `PlayFromStart` :!label _label)
      (:`Update`
        (`SceneComponent.K2_SetRelativeRotation` (`self.DoorPivot`) (`KismetMathLibrary.MakeRotator` 0.0 0.0 (* _newtrack_0 -90.0)) false false)
        (set `self.HasBeenUnlocked` true))
      (:`Finished`
        (`KismetSystemLibrary.PrintString` "Door is open!!" true true (struct :`G` 1.0 :`B` 0.322963 :`A` 1.0) 0.5)
        (`ActorComponent.K2_DestroyComponent` (`self.Sphere`))))
    (else
      (`KismetSystemLibrary.PrintString` "Get More Keys! Door is locked" true true (struct :`R` 0.479167 :`G` 0.051103 :`A` 1.0) 5.0)
      (if (`self.HasBeenUnlocked`)
        _
        (elif (not (`self.hasPlayedSound`))
          (`GameplayStatics.PlaySoundAtLocation` "/Game/Audio/locked_door_sound_1_Cue.locked_door_sound_1_Cue" (`SceneComponent.K2_GetComponentLocation` (`self.DefaultSceneRoot`)) (struct) 1.0 1.0 0.0 null null null null)
          (set `self.hasPlayedSound` true)
          (`KismetSystemLibrary.Delay` 1.0)
          (set `self.hasPlayedSound` false))))))

(event `self.Sphere.OnComponentEndOverlap`
  (params (OverlappedComponent :type "PrimitiveComponent Object Reference") (OtherActor :type "Actor Object Reference") (OtherComp :type "PrimitiveComponent Object Reference") (OtherBodyIndex :type Integer))
  (cast `/Game/Blueprints/BP_ThirdPersonCharacterCustom` OtherActor)
  (goto _label :!via `Stop`))

(fn `UserConstructionScript`)