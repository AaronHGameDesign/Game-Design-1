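; BP_ChestLidOpen is a locked chest that spends one key from the third-person character to open when that character enters its trigger.
; A timeline rotates the hinge with an opening sound, then prints a message and destroys the trigger.
; Without keys it prints a warning and plays a locked sound.
; Leaving the trigger stops the lid mid-swing, and re-entering costs another key to resume.
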(event `self.Trigger.OnComponentBeginOverlap`
  (params (OverlappedComponent :type "PrimitiveComponent Object Reference") (OtherActor :type "Actor Object Reference") (OtherComp :type "PrimitiveComponent Object Reference") (OtherBodyIndex :type Integer) (bFromSweep :type Boolean) (SweepResult :type "HitResult Structure (by ref)"))
  (bind _asbp_third_person_character_custom (cast `/Game/Blueprints/BP_ThirdPersonCharacterCustom` OtherActor))
  (bind _key_count (`/Game/Blueprints/BP_ThirdPersonCharacterCustom.Key Count` _asbp_third_person_character_custom))
  (if (> _key_count 0)
    (set `/Game/Blueprints/BP_ThirdPersonCharacterCustom.Key Count` (- _key_count 1) _asbp_third_person_character_custom) ; Remove a Key, then open door.
    (`GameplayStatics.PlaySoundAtLocation` "/Game/Audio/Chest_Opening_with_magic_sound_Cue.Chest_Opening_with_magic_sound_Cue" (`SceneComponent.K2_GetComponentLocation` (`self.DefaultSceneRoot`)) (struct) 1.0 1.0 0.0 null null null null)
    (bind (_direction _newtrack_0) (`Timeline|Open Chest Lid` :!label _label)
      (:`Update`
        (`SceneComponent.K2_SetRelativeRotation` (`self.Hinge`) (`KismetMathLibrary.MakeRotator` (* _newtrack_0 -90.0)) false false)
        (set `self.alreadyOpen` false))
      (:`Finished`
        (`KismetSystemLibrary.PrintString` "Chest is open!" true true (struct :`R` 0.191087 :`G` 1.0 :`B` 0.199986 :`A` 1.0))
        (`ActorComponent.K2_DestroyComponent` (`self.Trigger`))))
    (else
      (`KismetSystemLibrary.PrintString` "Get More Keys! The Chest is locked" true true (struct :`R` 0.479167 :`G` 0.051103 :`A` 1.0) 5.0)
      (if (not (`self.alreadyOpen`))
        (`GameplayStatics.PlaySoundAtLocation` "/Game/Audio/Chest_Locked.Chest_Locked" (`SceneComponent.K2_GetComponentLocation` (`self.DefaultSceneRoot`)) (struct) 1.0 1.0 0.0 null null null null)))))

(event `self.Trigger.OnComponentEndOverlap`
  (params (OverlappedComponent :type "PrimitiveComponent Object Reference") (OtherActor :type "Actor Object Reference") (OtherComp :type "PrimitiveComponent Object Reference") (OtherBodyIndex :type Integer))
  (cast `/Game/Blueprints/BP_ThirdPersonCharacterCustom` OtherActor)
  (goto _label :!via `Stop`))

(fn `UserConstructionScript`)