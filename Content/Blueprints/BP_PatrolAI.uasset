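; BP_PatrolAI is an AI character that wanders between tagged patrol points at a randomized walk speed.
; BeginPlay gathers and shuffles the tagged actors, then starts a self-repeating AIMoveTo loop that advances after success or failure, pauses, and reshuffles after each full pass.
; A separate GoToDestination event repeatedly chases the player until a move fails, but nothing in this file calls it.
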(event `self.ReceiveBeginPlay`
  ;[0.1896 1 0.498] Begin Play
  (bind _outactors (`GameplayStatics.GetAllActorsOfClassWithTag` "/Script/Engine.Actor" (`self.Patrol Point Tag`)))
  (`KismetSystemLibrary.PrintString` (`KismetStringLibrary.Concat_StrStr` "There are " (`KismetStringLibrary.Conv_IntToString` (`KismetArrayLibrary.Array_Length` _outactors)) " patrol points.") true true (struct :`R` 0.318274 :`G` 1.0 :`B` 0.163288 :`A` 1.0))
  (`KismetArrayLibrary.Array_Shuffle` _outactors)
  (set `CharacterMovementComponent.MaxWalkSpeed` (`KismetMathLibrary.Conv_IntToDouble` (* (`KismetMathLibrary.RandomIntegerInRange` 3 5) 25)) (`self.CharacterMovement`))
  (`self.GoToPatrolPoint`))

(event `GoToPatrolPoint`
  ;[1 0.9184 0.3915] Patrol
  (`|AIMoveTo` self (`self.K2_GetActorLocation` (`|GetArrayItem` (stale `self.ReceiveBeginPlay` _outactors) (`self.CurrentPatrolPoint`))) null 50.0
    (:`OnSuccess`
      (`KismetSystemLibrary.PrintString` "Arrived at Destination." true true (struct :`G` 1.0 :`B` 0.16855 :`A` 1.0)))
    (:`OnFail`
      (`KismetSystemLibrary.PrintString` "Failed to get to Destination." true true (struct :`R` 0.260417 :`B` 0.009499 :`A` 1.0))))
  (bind _result (`/Engine/EditorBlueprintResources/StandardMacros.IncrementInt` (`self.CurrentPatrolPoint`))
    (:`  `
      (if (>= _result (`KismetArrayLibrary.Array_Length` (stale `self.ReceiveBeginPlay` _outactors)))
        (set `self.CurrentPatrolPoint` 0)
        (`KismetArrayLibrary.Array_Shuffle` (stale `self.ReceiveBeginPlay` _outactors)))
      (`KismetSystemLibrary.Delay` 1.0)
      (`self.GoToPatrolPoint`))))

(event `GoToDestination`
  ;[1 0.1813 0.1116] Go To Player
  (`|AIMoveTo` self (0.0 0.0 0.0) (`GameplayStatics.GetPlayerCharacter` 0) 50.0
    (:`OnSuccess`
      (`KismetSystemLibrary.PrintString` "Arrived at Destination." true true (struct :`G` 1.0 :`B` 0.16855 :`A` 1.0))
      (`KismetSystemLibrary.Delay` 1.0)
      (`self.GoToDestination`))
    (:`OnFail`
      (`KismetSystemLibrary.PrintString` "Failed to get to Destination." true true (struct :`R` 0.260417 :`B` 0.009499 :`A` 1.0)))))

(fn `UserConstructionScript`)