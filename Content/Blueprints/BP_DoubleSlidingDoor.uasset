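; BP_DoubleSlidingDoor is a two-panel door that slides when something overlaps its Trigger component and slides back when an overlap ends.
; The Slide timeline plays on begin overlap and reverses on end overlap, with no filtering or counting of overlapping actors.
; Each update lerps LeftDoor and RightDoor relative locations between their Current and New vector variables, without sweep.
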(event `self.Trigger.OnComponentBeginOverlap`
  (params (OverlappedComponent :type "PrimitiveComponent Object Reference") (OtherActor :type "Actor Object Reference") (OtherComp :type "PrimitiveComponent Object Reference") (OtherBodyIndex :type Integer) (bFromSweep :type Boolean) (SweepResult :type "HitResult Structure (by ref)"))
  (bind (_direction _slide) (`Timeline|Slide` :!label _label)
    (:`Update`
      (`|ExecutionSequence`
        (:`then_0`
          (`SceneComponent.K2_SetRelativeLocation` (`self.LeftDoor`) (`KismetMathLibrary.VLerp` (`self.CurrentLeft`) (`self.NewLeft`) _slide) false false))
        (:`then_1`
          (`SceneComponent.K2_SetRelativeLocation` (`self.RightDoor`) (`KismetMathLibrary.VLerp` (`self.CurrentRight`) (`self.NewRight`) _slide) false false))))))

(event `self.Trigger.OnComponentEndOverlap`
  (params (OverlappedComponent :type "PrimitiveComponent Object Reference") (OtherActor :type "Actor Object Reference") (OtherComp :type "PrimitiveComponent Object Reference") (OtherBodyIndex :type Integer))
  (goto _label :!via `Reverse`))

(fn `UserConstructionScript`)