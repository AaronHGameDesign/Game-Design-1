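; Enemy Blueprint that moves toward the player character once its PawnSensing component sees a pawn.
; Sensing sets IsSeenPlayer, which nothing here clears, and calls FollowPlayer to issue an AI MoveTo on the first player's character.
; A separate GoToDestination event makes the same move, repeating after a short delay on success and only printing on failure; nothing else in this graph calls it.
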(event `self.PawnSensing.OnSeePawn`
  (params (Pawn :type "Pawn Object Reference"))
  (set `self.IsSeenPlayer` true)
  (`self.FollowPlayer`))

(event `FollowPlayer`
  (if (`self.IsSeenPlayer`)
    (`|AIMoveTo` self (0.0 0.0 0.0) (`GameplayStatics.GetPlayerCharacter` 0) 50.0)))

(event `GoToDestination`
  ;[1 0.1813 0.1116] Go To Player
  (`|AIMoveTo` self (0.0 0.0 0.0) (`GameplayStatics.GetPlayerCharacter` 0) 50.0
    (:`OnSuccess`
      (`KismetSystemLibrary.PrintString` "Arrived at Destination." true true (struct :`G` 1.0 :`B` 0.16855 :`A` 1.0))
      (`KismetSystemLibrary.Delay` 1.0)
      (`self.GoToDestination`))
    (:`OnFail`
      (`KismetSystemLibrary.PrintString` "Failed to get to Destination." true true (struct :`R` 0.260417 :`B` 0.009499 :`A` 1.0)))))

(fn `UserConstructionScript`)